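; Player-controlled hover boat with a rotating turret and switchable missile weapons.
; Four hover components act on a physics base, driven by forward force and yaw input while a downward trace hits a surface.
; Firing applies recoil and launches the selected missile along camera rotation via BPI_Missiles, with a DoOnce and delay limiting fire rate.
; Tab cycles basic, gatling and sniping missiles, setting turret mesh, missile class and fire rate.
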(event `self.ReceiveBeginPlay`
  (`/Game/Assets/HoverComponent.InitComponent` (`self.HoverComponent2`) (`self.BoatPhysicsBase`))
  (`/Game/Assets/HoverComponent.InitComponent` (`self.HoverComponent1`) (`self.BoatPhysicsBase`))
  (`/Game/Assets/HoverComponent.InitComponent` (`self.HoverComponent`) (`self.BoatPhysicsBase`))
  (`/Game/Assets/HoverComponent.InitComponent` (`self.HoverComponent3`) (`self.BoatPhysicsBase`))
  (bind _ascustom_game_mode (cast `/Game/Blueprints/CustomGameMode` (`GameplayStatics.GetGameMode`))
    (:`then`
      (set `self.GameMode` _ascustom_game_mode)
      (set `self.Health` (`/Game/Blueprints/CustomGameMode.PlayerStartingHealth` (`self.GameMode`)))
      (`self.SelectMissile` "NewEnumerator0"))
    (:`CastFailed`
      (`KismetSystemLibrary.PrintString` "BP_Boat: Cast to GM Failed"))))

(event `InputAxis|MoveForward`
  (params (AxisValue :type "Float (single-precision)"))
  (bind _boatphysicsbase (`self.BoatPhysicsBase`))
  (if (`self.CanMove`)
    (`PrimitiveComponent.AddForce` _boatphysicsbase (* (* (`SceneComponent.GetForwardVector` _boatphysicsbase) (* (`self.ForwardSpeed`) (`self.NormalizePhysicsValue`))) AxisValue) "None" false)))

(event `InputAxis|MoveRight`
  (params (AxisValue :type "Float (single-precision)"))
  (if (`self.CanMove`)
    (`SceneComponent.K2_AddLocalRotation` (`self.BoatPhysicsBase`) (`KismetMathLibrary.MakeRotator` 0.0 0.0 (* AxisValue (`self.YawPerSec`))) false false)))

(event `InputAxis|Turn`
  (params (AxisValue :type "Float (single-precision)"))
  (`SceneComponent.K2_AddLocalRotation` (`self.SM_Boat_CH_BoatTurret`) (`KismetMathLibrary.MakeRotator` 0.0 0.0 (* AxisValue (`self.CameraTurnRate`))) false false))

(event `InputAxis|LookUp`
  (params (AxisValue :type "Float (single-precision)"))
  (bind _springarm (`self.SpringArm`))
  (bind (_returnvalue_roll _returnvalue_pitch) (`KismetMathLibrary.BreakRotator` (`SpringArmComponent.GetTargetRotation` _springarm)))
  (`SceneComponent.K2_AddLocalRotation` _springarm (`KismetMathLibrary.MakeRotator` 0.0 (* AxisValue (`self.CameraTurnRate`))) false false)
  (`SceneComponent.K2_SetRelativeRotation` _springarm (`KismetMathLibrary.MakeRotator` 0.0 (`KismetMathLibrary.FClamp` _returnvalue_pitch -89.0 -10.0)) false false))

(event `InputAction|Fire`
  (params (Key :type "Key Structure"))
  (bind _camera (`self.Camera`))
  (bind _returnvalue (`SceneComponent.K2_GetComponentLocation` (`self.FirePosition`)))
  (bind _returnvalue_2 (`SceneComponent.K2_GetComponentRotation` _camera))
  (:`Pressed`
    (`/Engine/EditorBlueprintResources/StandardMacros.DoOnce` false :!label _label
      (:`Completed`
        ;[1 1 1] Recoil: Get the turrets forward vector and reverse it + Add force in that direction
        (`PrimitiveComponent.AddForce` (`self.BoatPhysicsBase`) (* (* (`SceneComponent.GetForwardVector` (`self.SM_Boat_CH_BoatTurret`)) -1.0) (* (`self.RecoilForce`) (`self.NormalizePhysicsValue`))) "None" false)
        ;[1 1 1] Projectile aim path: Gets the turrets fire position, and the position the centre of the camera is looking
        (`KismetSystemLibrary.LineTraceSingle` :`Start` _returnvalue :`End` (+ (`SceneComponent.K2_GetComponentLocation` _camera) (* (`KismetMathLibrary.GetForwardVector` _returnvalue_2) 3000.0)) :`TraceChannel` "TraceTypeQuery1" :`DrawDebugType` "ForOneFrame")
        (bind _returnvalue_3 (`|SpawnActorFromClass` (`self.MissileType`) (`KismetMathLibrary.MakeTransform` _returnvalue _returnvalue_2) "Undefined" "OverrideRootScale" null null))
        (if (`KismetSystemLibrary.DoesImplementInterface` _returnvalue_3 "/Game/Blueprints/BPI_Missiles.BPI_Missiles_C")
          (message `/Game/Blueprints/BPI_Missiles.Launch` _returnvalue_3)
          (`KismetSystemLibrary.Delay` (`self.RateOfFire`))
          (goto _label :!via `Reset`)
          (else
            (`KismetSystemLibrary.PrintString` "BP_Boat: Missile lacks interface")))))))

(event `InputAxis|HoldFire`
  (params (AxisValue :type "Float (single-precision)"))
  (if (`KismetMathLibrary.NearlyEqual_FloatFloat` AxisValue 1.0 0.1)
    (goto _label)))

(event `self.ReceiveTick`
  (params (DeltaSeconds :type "Float (single-precision)"))
  (bind _returnvalue (`SceneComponent.K2_GetComponentLocation` (`self.BoatPhysicsBase`)))
  (bind (_outhit _returnvalue_2) (`KismetSystemLibrary.LineTraceSingle` :`Start` _returnvalue :`End` (+ _returnvalue (0.0 0.0 -200.0)) :`TraceChannel` "TraceTypeQuery1" :`DrawDebugType` "ForOneFrame"))
  (set `self.CanMove` _returnvalue_2))

(event `Key|Tab`
  (params (Key :type "Key Structure"))
  ;[1 1 1] Cycle through weapons
  (:`Pressed`
    (`/Engine/EditorBlueprintResources/StandardMacros.IncrementInt` (`self.CurrentGun`)
      (:`  `
        (`self.SelectMissile` (cast `/Game/Blueprints/E_EquippedMissile` (mod (`KismetMathLibrary.Conv_IntToByte` (mod (`self.CurrentGun`) 255)) (+ (`self.MaxGun`) 1))))))))

(event `SelectMissile`
  (params (Selection :type "/Game/Blueprints/E_EquippedMissile Enum" :default "NewEnumerator0"))
  (switch `/Game/Blueprints/E_EquippedMissile` Selection
    (:`NewEnumerator0`
      ;[1 1 1] Base Missle
      (`StaticMeshComponent.SetStaticMesh` (`self.SM_Boat_CH_BoatTurret`) "/Game/Assets/Gun1_NoTXT.Gun1_NoTXT")
      (set `self.MissileType` "/Game/Blueprints/BP_MissileBase.BP_MissileBase_C")
      (set `self.RateOfFire` 0.5))
    (:`NewEnumerator1`
      ;[1 1 1] Gatling Missile
      (`StaticMeshComponent.SetStaticMesh` (`self.SM_Boat_CH_BoatTurret`) null)
      (set `self.MissileType` "/Game/Blueprints/BP_MissileGatling.BP_MissileGatling_C")
      (set `self.RateOfFire` 0.2))
    (:`NewEnumerator2`
      ;[1 1 1] Sniping Missile
      (`StaticMeshComponent.SetStaticMesh` (`self.SM_Boat_CH_BoatTurret`) "/Game/Assets/Gun2_NoTXT.Gun2_NoTXT")
      (set `self.MissileType` "/Game/Blueprints/BP_MissileSniping.BP_MissileSniping_C")
      (set `self.RateOfFire` 1.0))))

(fn `UserConstructionScript`)