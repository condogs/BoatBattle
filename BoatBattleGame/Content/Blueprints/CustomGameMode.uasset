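; Game mode for a local multiplayer boat game that creates players and swaps their pawns.
; On BeginPlay it caches all PlayerStarts and creates local players in a loop capped by a player counter.
; SpawnCharacter replaces a controller's current pawn with a possessed BP_Boat, while DespawnPlayer swaps it back to InitPawn.
; Both spawn at a randomly chosen PlayerStart and act only when a valid pawn is already controlled.
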(event `self.ReceiveBeginPlay`
  (bind _numberofplayers (`self.NumberOfPlayers`))
  (bind _outactors (`GameplayStatics.GetAllActorsOfClass` "/Script/Engine.PlayerStart"))
  (set `self.SpawnPoints` _outactors)
  (while (<= _numberofplayers 3)
    (set `self.NumberOfPlayers` (+ _numberofplayers 1))
    (`GameplayStatics.CreatePlayer` -1)))

(event `SpawnCharacter`
  (params (PlayerController :type "PlayerController Object Reference"))
  (bind _returnvalue (`Controller.K2_GetPawn` PlayerController))
  (`/Engine/EditorBlueprintResources/StandardMacros.IsValid` _returnvalue
    (:`Is Valid`
      (`self.K2_DestroyActor` _returnvalue)
      (`|SpawnActorFromClass` "/Game/Blueprints/BP_Boat.BP_Boat_C" (`self.GetRandomSpawn`) "Undefined" "OverrideRootScale" null null)
      (`Controller.Possess` PlayerController null))))

(event `DespawnPlayer`
  (params (PlayerController :type "PlayerController Object Reference"))
  (bind _returnvalue (`Controller.K2_GetPawn` PlayerController))
  (`/Engine/EditorBlueprintResources/StandardMacros.IsValid` _returnvalue
    (:`Is Valid`
      (`self.K2_DestroyActor` _returnvalue)
      (`|SpawnActorFromClass` "/Game/Blueprints/InitPawn.InitPawn_C" (`self.GetRandomSpawn`) "Undefined" "OverrideRootScale" null null)
      (`Controller.Possess` PlayerController null))))

(fn `UserConstructionScript`)