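; Player controller Blueprint that lets a player request a character spawn or despawn from the game mode.
; Space Bar or Gamepad Special Left calls SpawnCharacter on CustomGameMode, while Backspace or Gamepad Special Right calls DespawnPlayer.
; Both calls pass the controller itself, leaving the spawn and despawn logic to the game mode.
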(event `Key|Gamepad_Special_Left`
  (params (Key :type "Key Structure"))
  (:`Pressed`
    (bind _ascustom_game_mode (cast `/Game/Blueprints/CustomGameMode` (`GameplayStatics.GetGameMode`) :!label _label))
    (`/Game/Blueprints/CustomGameMode.SpawnCharacter` _ascustom_game_mode self)))

(event `Key|SpaceBar`
  (params (Key :type "Key Structure"))
  (:`Pressed`
    (goto _label)))

(event `Key|BackSpace`
  (params (Key :type "Key Structure"))
  (:`Pressed`
    (bind _ascustom_game_mode (cast `/Game/Blueprints/CustomGameMode` (`GameplayStatics.GetGameMode`) :!label _label_2))
    (`/Game/Blueprints/CustomGameMode.DespawnPlayer` _ascustom_game_mode self)))

(event `Key|Gamepad_Special_Right`
  (params (Key :type "Key Structure"))
  (:`Pressed`
    (goto _label_2)))

(fn `UserConstructionScript`)