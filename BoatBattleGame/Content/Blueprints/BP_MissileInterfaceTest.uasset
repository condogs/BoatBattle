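; BP_MissileInterfaceTest is a test missile actor that is fired through a Launch event and reacts to what it hits.
; Launch calls ShootProjectile on the Cube mesh, passing the Scene component for orientation and a configurable force.
; A timer set on BeginPlay destroys the actor after its lifetime.
; Hits print debug success or fail, and only Pawn hits activate the explosion effect without destroying the missile.
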(event `/Game/Blueprints/BPI_Missiles.Launch`
  ;[1 1 1] Shooting
  (`/Game/Blueprints/BPFL_LukasAssorted.ShootProjectile` (`self.Cube`) (`self.Scene`) (`self.MissileForce`)))

(event `DestroySelf`
  ;[1 1 1] Destroy Projectile after  X Seconds
  (`self.K2_DestroyActor`))

(event `self.ReceiveBeginPlay`
  (`|ExecutionSequence`
    (:`then_0`
      ;[1 1 1] Destroy Projectile after  X Seconds
      (`KismetSystemLibrary.K2_SetTimerDelegate` (delegate `DestroySelf`) (`self.ProjectileLifetime`)))))

(event `self.ReceiveHit`
  (params (MyComp :type "PrimitiveComponent Object Reference") (Other :type "Actor Object Reference") (OtherComp :type "PrimitiveComponent Object Reference") (bSelfMoved :type Boolean) (HitLocation :type "Vector Structure") (HitNormal :type "Vector Structure") (NormalImpulse :type "Vector Structure") (Hit :type "HitResult Structure (by ref)"))
  (cast `Pawn` Other
    (:`then`
      (`KismetSystemLibrary.PrintString` "success")
      (`ActorComponent.Activate` (`self.PS_Explosion`) false))
    (:`CastFailed`
      (`KismetSystemLibrary.PrintString` "fail"))))

(fn `UserConstructionScript`)